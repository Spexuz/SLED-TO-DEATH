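; Player character Blueprint with axis-driven movement and a physics-simulated mesh using physical animation.
; BeginPlay sets up mesh simulation and applies the FullBodyProfile physical animation profile.
; Movement axes feed AddMovementInput along the actor's forward and right vectors.
; Two RagDollToggle handlers change mesh simulation, one also setting root-bone bodies and blend weight, but both branch on a constant true, so neither alternates.
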(event `self.ReceiveBeginPlay`
  (`PrimitiveComponent.SetSimulatePhysics` (`self.Mesh`) (`self.SimulateOn`))
  (`SkeletalMeshComponent.SetAllBodiesBelowSimulatePhysics` (`self.Mesh`) (`self.In Bone Name`) false true)
  (set `self.SimulateOn` true)
  (`PrimitiveComponent.SetSimulatePhysics` (`self.Mesh`) (`self.SimulateOn`))
  (`PhysicalAnimationComponent.ApplyPhysicalAnimationProfileBelow` (`self.PhysicalAnimation`) "FullBodyProfile" "FullBodyProfile" true false))

(event `InputAxis|MoveRight`
  (params (AxisValue :type "Float (single-precision)")))

(event `InputAction|RagDollToggle`
  (params (Key :type "Key Structure"))
  (:`Pressed`
    (if true
      (`PrimitiveComponent.SetSimulatePhysics` (`self.Mesh`) true)
      (else
        (`PrimitiveComponent.SetSimulatePhysics` (`self.Mesh`) false)))))

(event `InputAxis|MoveBack`
  (params (AxisValue :type "Float (single-precision)"))
  (`self.AddMovementInput` (`self.GetActorForwardVector`) AxisValue))

(event `InputAxis|MoveForward`
  (params (AxisValue :type "Float (single-precision)"))
  (`self.AddMovementInput` (`self.GetActorForwardVector`) AxisValue))

(event `InputAxis|MoveLeft`
  (params (AxisValue :type "Float (single-precision)"))
  (`self.AddMovementInput` (`self.GetActorRightVector`) AxisValue))

(event `InputAction|RagDollToggle`
  (params (Key :type "Key Structure"))
  (:`Pressed`
    (if true
      (`PrimitiveComponent.SetSimulatePhysics` (`self.Mesh`) false)
      (`SkeletalMeshComponent.SetAllBodiesBelowSimulatePhysics` (`self.Mesh`) (`SkinnedMeshComponent.GetBoneName` (`self.Mesh`) 0) false true)
      (`SkeletalMeshComponent.SetPhysicsBlendWeight` (`self.Mesh`) 1.0)
      (else
        (`PrimitiveComponent.SetSimulatePhysics` (`self.Mesh`) true)
        (`SkeletalMeshComponent.SetAllBodiesBelowSimulatePhysics` (`self.Mesh`) (`SkinnedMeshComponent.GetBoneName` (`self.Mesh`) 0) true true)
        (`SkeletalMeshComponent.SetPhysicsBlendWeight` (`self.Mesh`) 0.3)))))

(event `InputAxis|MoveRight`
  (params (AxisValue :type "Float (single-precision)"))
  (`self.AddMovementInput` (`self.GetActorRightVector`) AxisValue))

(fn `UserConstructionScript`)